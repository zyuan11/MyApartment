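; bp_AlterMenu is an actor that holds a set of five objects for a menu.
; On BeginPlay, InitObjs gathers the five object variables into the Objs array.
; Two helper functions convert a scale to a normalized menu size and back using a fixed target ratio, though neither is called within this Blueprint.
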(event `self.ReceiveBeginPlay`
  (`self.InitObjs`))

(fn `InitObjs`
  (bind _objs (`self.Objs`))
  (`|ExecutionSequence`
    (:`then_0`
      (`KismetArrayLibrary.Array_Add` _objs (`self.Obj0`)))
    (:`then_1`
      (`KismetArrayLibrary.Array_Add` _objs (`self.Obj1`)))
    (:`then_2`
      (`KismetArrayLibrary.Array_Add` _objs (`self.Obj2`)))
    (:`then_3`
      (`KismetArrayLibrary.Array_Add` _objs (`self.Obj3`)))
    (:`then_4`
      (`KismetArrayLibrary.Array_Add` _objs (`self.Obj4`))
      (return))))

(fn `RescaleObjForMenu`
  (params (ObjScale :type "Float (double-precision)") (Scale_i :type "Vector Structure"))
  (returns (NewScale :type "Vector Structure"))
  (return (* Scale_i (/ 0.2 ObjScale))))

(fn `RescaleObjForMenu_Back`
  (params (ObjScale_i :type "Float (double-precision)") (scale_i :type "Vector Structure"))
  (returns (scale_o :type "Vector Structure"))
  (return (/ scale_i (/ 0.2 ObjScale_i))))

(fn `UserConstructionScript`)