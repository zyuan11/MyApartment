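; Inventory of furniture and materials, each represented by a spawned BP_UserInterface preview actor tagged by category.
; Furniture previews copy a rescaled mesh and material, material previews use a cube, and maps link each to its class or material.
; Previews stay hidden and are toggled on or off by category queries and returns, rather than respawned.
; InventoryDispatching adds hardcoded debug floor and wall materials, then fires the load dispatcher for new items.
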(fn `AddFurniture`
  (params (FurnitureReference :type "/Game/Blueprints/BP_Furniture_old Object Reference"))
  (bind _staticmesh (`/Game/Blueprints/BP_Furniture_old.StaticMesh` FurnitureReference))
  (`|ExecutionSequence`
    (:`then_0`
      (bind _resizedtransform (`self.CalculateTransform` FurnitureReference))
      (bind _returnvalue (`|SpawnActorFromClass` "/Game/Blueprints/BP_UserInterface.BP_UserInterface_C" _resizedtransform "AlwaysSpawn" "OverrideRootScale"))
      (bind _staticmesh_2 (`/Game/Blueprints/BP_UserInterface.StaticMesh` _returnvalue))
      (bind _returnvalue_2 (`StaticMeshComponent.SetStaticMesh` _staticmesh_2 (`StaticMeshComponent.StaticMesh` _staticmesh)))
      (if _returnvalue_2
        (`PrimitiveComponent.SetMaterial` _staticmesh_2 0 (`PrimitiveComponent.GetMaterial` _staticmesh 0))
        (bind _reference (`self.EnableUI` _returnvalue))
        (bind _output_get (set `Actor.Tags` (`Actor.Tags` FurnitureReference) _reference))
        (`BlueprintSetLibrary.Set_Add` (`self.FurnitureCategories`) (`KismetArrayLibrary.Array_Get` _output_get 1))))
    (:`then_1`
      (if _returnvalue_2
        (bind _returnvalue_3 (`BlueprintSetLibrary.Set_Add` (`self.InventoryStack`) _returnvalue))
        (if _returnvalue_3
          (`BlueprintMapLibrary.Map_Add` (`self.FurnitureMap`) _returnvalue (`GameplayStatics.GetObjectClass` FurnitureReference)))))
    (:`then_2`
      (set `self.NewItemInserted` true))))

(fn `AddMaterial`
  (params (MaterialReference :type "MaterialInterface Object Reference") (Category :type Name))
  (locals (DefaultTransform :type "Transform Structure" :default "0.000000,0.000000,0.000000|0.000000,0.000000,0.000000|0.100000,0.100000,0.100000"))
  (`|ExecutionSequence`
    (:`then_0`
      (bind _returnvalue (`|SpawnActorFromClass` "/Game/Blueprints/BP_UserInterface.BP_UserInterface_C" (`local.DefaultTransform`) "AlwaysSpawn" "OverrideRootScale"))
      (bind _returnvalue_2 (`StaticMeshComponent.SetStaticMesh` (`/Game/Blueprints/BP_UserInterface.StaticMesh` _returnvalue) "/Game/Geometry/Meshes/1M_Cube.1M_Cube"))
      (if _returnvalue_2
        (`PrimitiveComponent.SetMaterial` (`/Game/Blueprints/BP_UserInterface.StaticMesh` _returnvalue) 0 MaterialReference)
        (`self.EnableUI` _returnvalue)
        (set `Actor.Tags` (`|MakeArray` Category) _returnvalue)))
    (:`then_1`
      (if _returnvalue_2
        (bind _returnvalue_3 (`BlueprintSetLibrary.Set_Add` (`self.InventoryStack`) _returnvalue))
        (if _returnvalue_3
          (`BlueprintMapLibrary.Map_Add` (`self.MaterialMap`) _returnvalue MaterialReference))))
    (:`then_2`
      (set `self.NewItemInserted` true))))

(fn `CalculateTransform`
  (params (FurnitureReference :type "/Game/Blueprints/BP_Furniture_old Object Reference"))
  (returns (ResizedTransform :type "Transform Structure"))
  (locals (DefaultLocation :type "Vector Structure" :default (0.0 0.0 -200.0)) (TargetSize :type "Vector Structure" :default (10.0 10.0 10.0)) (DefaultRotation :type "Rotator Structure"))
  (return (`KismetMathLibrary.MakeTransform` (`local.DefaultLocation`) (`local.DefaultRotation`) (/ (`local.TargetSize`) (* (`.BoxExtent` (`Actor.GetActorBounds` FurnitureReference false)) 2)))))

(fn `EnableUI`
  (params (UIReference :type "/Game/Blueprints/BP_UserInterface Object Reference") (Enable :type Boolean))
  (returns (Reference :type "/Game/Blueprints/BP_UserInterface Object Reference"))
  (`Actor.SetActorEnableCollision` UIReference Enable)
  (`Actor.SetActorTickEnabled` UIReference Enable)
  (`Actor.SetActorHiddenInGame` UIReference (not Enable))
  (return UIReference))

(fn `GetFurnitureCategories`
  (returns (Categories :type "Array of Name"))
  (bind _result (`BlueprintSetLibrary.Set_ToArray` (`self.FurnitureCategories`)))
  (return _result))

(fn `GetFurnitureClass`
  (params (UIReference :type "/Game/Blueprints/BP_UserInterface Object Reference"))
  (returns (FurnitureClass :type "/Game/Blueprints/BP_Furniture_old Class Reference"))
  (bind (_value _returnvalue) (`BlueprintMapLibrary.Map_Find` (`self.FurnitureMap`) UIReference))
  (if _returnvalue
    (return _value)
    (else
      (return null))))

(fn `GetFurnitureReferences`
  (params (Category :type Name))
  (returns (FurnitureReference :type "/Game/Blueprints/BP_Furniture_old Class Reference"))
  (bind _furnituremap (`self.FurnitureMap`))
  (bind _keys (`BlueprintMapLibrary.Map_Keys` _furnituremap))
  (for _array_element _keys
    (if (`Actor.ActorHasTag` _array_element Category)
      (break)))
  (return (`BlueprintMapLibrary.Map_Find` _furnituremap _array_element)))

(fn `GetFurnitureUIElements`
  (params (Category :type Name) (NumberOfItems :type Integer))
  (returns (UIEelements :type "Array of /Game/Blueprints/BP_UserInterface Object Reference"))
  (locals (UIReferences :type "Array of /Game/Blueprints/BP_UserInterface Object Reference"))
  (bind _uireferences (`local.UIReferences`))
  (bind _result (`BlueprintSetLibrary.Set_ToArray` (`self.InventoryStack`)))
  (for _array_element _result
    (if (`Actor.ActorHasTag` _array_element Category)
      (bind _reference (`self.EnableUI` _array_element true))
      (`KismetArrayLibrary.Array_Add` _uireferences _reference)
      (if (== (`KismetArrayLibrary.Array_Length` _uireferences) NumberOfItems)
        (break))))
  (return (`local.UIReferences`)))

(fn `GetInventoryStatus`
  (returns (InventoryStatus :type Boolean))
  (return (`self.NewItemInserted`)))

(fn `GetMaterialReference`
  (params (Category :type Name))
  (returns (Material :type "MaterialInterface Object Reference"))
  (locals (FoundItem :type Boolean))
  (bind _materialmap (`self.MaterialMap`))
  (bind _keys (`BlueprintMapLibrary.Map_Keys` _materialmap))
  (if (> (`KismetArrayLibrary.Array_Length` _keys) 0)
    (for _array_element _keys
      (if (`Actor.ActorHasTag` _array_element Category)
        (set `local.FoundItem` true)
        (break)))
    (bind (_value _returnvalue) (`BlueprintMapLibrary.Map_Find` _materialmap _array_element))
    (if (and _returnvalue (`local.FoundItem`))
      (return _value)
      (else
        (return null)))
    (else
      (return null))))

(fn `GetMaterialUIElements`
  (params (Category :type Name) (NumberOfElements :type Integer))
  (returns (UIReferences :type "Array of /Game/Blueprints/BP_UserInterface Object Reference"))
  (locals (UIElements :type "Array of /Game/Blueprints/BP_UserInterface Object Reference"))
  (bind _uielements (`local.UIElements`))
  (bind _keys (`BlueprintMapLibrary.Map_Keys` (`self.MaterialMap`)))
  (for _array_element _keys
    (if (`Actor.ActorHasTag` _array_element Category)
      (bind _reference (`self.EnableUI` _array_element true))
      (`KismetArrayLibrary.Array_Add` _uielements _reference)
      (if (== (`KismetArrayLibrary.Array_Length` _uielements) NumberOfElements)
        (break))))
  (return (`local.UIElements`)))

(fn `GetMeterialInstance`
  (params (UIReference :type "/Game/Blueprints/BP_UserInterface Object Reference"))
  (returns (MaterialInstance :type "MaterialInterface Object Reference"))
  (bind (_value _returnvalue) (`BlueprintMapLibrary.Map_Find` (`self.MaterialMap`) UIReference))
  (if _returnvalue
    (return _value)
    (else
      (return null))))

(fn `InventoryDispatching`
  (`|ExecutionSequence`
    (:`then_0`
      ;[1 1 1] DEBUG
      (`self.AddMaterial` "/Game/Materials/Floor/M_WalnutFloor.M_WalnutFloor" "Floor")
      (`self.AddMaterial` "/Game/Materials/Floor/M_OakFloor.M_OakFloor" "Floor")
      (`self.AddMaterial` "/Game/StarterContent/Materials/M_Brick_Clay_New.M_Brick_Clay_New" "Wall"))
    (:`then_1`
      (if (`self.NewItemInserted`)
        (`self.LoadInventoryDispatcher`)
        (set `self.NewItemInserted` false)))))

(fn `PrintItems`
  (bind _furnituremap (`self.FurnitureMap`))
  (bind _materialmap (`self.MaterialMap`))
  (`|ExecutionSequence`
    (:`then_0`
      ;[1 1 1] Dump Inventory stack items
      (`KismetSystemLibrary.PrintString` "Dump InventoryStack")
      (bind _result (`BlueprintSetLibrary.Set_ToArray` (`self.InventoryStack`)))
      (for (_array_element _array_index) _result
        (`KismetSystemLibrary.PrintString` (`KismetStringLibrary.Concat_StrStr` "At index " (`KismetStringLibrary.Conv_IntToString` _array_index) (`KismetSystemLibrary.GetDisplayName` _array_element)))))
    (:`then_1`
      ;[1 1 1] Dump Inventory Funiture map
      (`KismetSystemLibrary.PrintString` "Dump FurnitureMap")
      (bind _keys (`BlueprintMapLibrary.Map_Keys` _furnituremap))
      (for (_array_element_2 _array_index_2) _keys
        (`KismetSystemLibrary.PrintString` (`KismetStringLibrary.Concat_StrStr` "At Index " (`KismetStringLibrary.Conv_IntToString` _array_index_2) "Key: " (`KismetSystemLibrary.GetDisplayName` _array_element_2) "Value: " (`KismetSystemLibrary.GetClassDisplayName` (`BlueprintMapLibrary.Map_Find` _furnituremap _array_element_2))))))
    (:`then_2`
      ;[1 1 1] Dump Inventory Material map
      (`KismetSystemLibrary.PrintString` "Dump MaterialMap")
      (bind _keys_2 (`BlueprintMapLibrary.Map_Keys` _materialmap))
      (for (_array_element_3 _array_index_3) _keys_2
        (`KismetSystemLibrary.PrintString` (`KismetStringLibrary.Concat_StrStr` "At Index " (`KismetStringLibrary.Conv_IntToString` _array_index_3) "Key: " (`KismetSystemLibrary.GetDisplayName` _array_element_3) "Value: " (`KismetSystemLibrary.GetDisplayName` (`BlueprintMapLibrary.Map_Find` _materialmap _array_element_3))))))
    (:`then_3`
      ;[1 1 1] Dump Furniture Categories
      (`KismetSystemLibrary.PrintString` "Dump Categories")
      (bind _result_2 (`BlueprintSetLibrary.Set_ToArray` (`self.FurnitureCategories`)))
      (for (_array_element_4 _array_index_4) _result_2
        (`KismetSystemLibrary.PrintString` (`KismetStringLibrary.Concat_StrStr` "At Index " (`KismetStringLibrary.Conv_IntToString` _array_index_4) (`KismetStringLibrary.Conv_NameToString` _array_element_4)))))))

(fn `ReturnFurnitureUI`
  (params (UIReferences :type "Array of /Game/Blueprints/BP_UserInterface Object Reference"))
  (for _array_element UIReferences
    (`self.EnableUI` _array_element)))