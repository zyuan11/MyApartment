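; Selectable furniture actor that can be moved and swapped for alternatives from the inventory.
; While selected it changes scale and offset and follows the controller's valid placement result each Tick, while hover toggles custom depth stencil highlighting on its meshes.
; It fetches option UI actors from BP_Inventory, cast from the GameInstance, by tag category and lines them up.
; Applying an option returns them, then spawns any different class in its place and destroys itself.
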(event `self.ReceiveBeginPlay`
  ;[1 1 1] Find Inventory
  (bind _asbp_inventory (cast `/Game/Blueprints/BP_Inventory` (`GameplayStatics.GetGameInstance`)))
  (set `self.InventoryReference` _asbp_inventory))

(event `self.ReceiveTick`
  (params (DeltaSeconds :type "Float (single-precision)"))
  (`self.UpdateLocation`))

(event `/Game/Blueprints/BP_ObjectInterface.Select`
  (params (ControllerReference :type "/Game/Blueprints/BP_ObjectController Object Reference"))
  ;[1 1 1] onSelect Implementation
  (`|ExecutionSequence`
    (:`then_0`
      (`self.SetActorRelativeScale3D` (`self.ObjectSelectedScale`))
      (`SceneComponent.K2_AddRelativeLocation` (`self.DefaultSceneRoot`) (`self.ObjectSelectedLocation`) false false))
    (:`then_1`
      (set `self.ObjController` ControllerReference)
      (set `self.Selected` true))))

(event `/Game/Blueprints/BP_ObjectInterface.Deselect`
  ;[1 1 1] onDeselect Implementation
  (`|ExecutionSequence`
    (:`then_0`
      (`self.SetActorRelativeScale3D` (* (`self.ObjectSelectedScale`) 2))
      (`SceneComponent.K2_AddRelativeLocation` (`self.DefaultSceneRoot`) (* (`self.ObjectSelectedLocation`) -1) false false))
    (:`then_1`
      (set `self.ObjController` null)
      (set `self.Selected` false))))

(event `/Game/Blueprints/BP_ObjectInterface.OnHover`
  ;[1 1 1] OnHover Implementation
  (for _array_element (`SceneComponent.GetChildrenComponents` (`self.DefaultSceneRoot`) false)
    (bind _asstatic_mesh_component (cast `StaticMeshComponent` _array_element))
    (`PrimitiveComponent.SetRenderCustomDepth` _asstatic_mesh_component true)
    (`PrimitiveComponent.SetCustomDepthStencilValue` _asstatic_mesh_component 3)))

(event `/Game/Blueprints/BP_ObjectInterface.ExitHover`
  ;[1 1 1] ExitHover Implementation
  (for _array_element (`SceneComponent.GetChildrenComponents` (`self.DefaultSceneRoot`) false)
    (bind _asstatic_mesh_component (cast `StaticMeshComponent` _array_element))
    (`PrimitiveComponent.SetRenderCustomDepth` _asstatic_mesh_component false)
    (`PrimitiveComponent.SetCustomDepthStencilValue` _asstatic_mesh_component 0)))

(event `/Game/Blueprints/BP_ObjectInterface.ApplyOptions`
  (params (CurrentUIReference :type Integer))
  (bind _item (`KismetArrayLibrary.Array_Get` (`self.UIElements`) CurrentUIReference))
  ;[1 1 1] Apply selected UI
  (if (== CurrentUIReference -1)
    (`self.ReturnUIOptions` :!label _label)
    (else
      (bind _furnitureclass (`/Game/Blueprints/BP_Inventory.GetFurnitureClass` (`self.InventoryReference`) _item))
      (if (== _furnitureclass (`GameplayStatics.GetObjectClass` self))
        (goto _label)
        (else
          (set `self.SelectedReference` _item)
          (`self.ReturnUIOptions`)
          (`self.ReplaceActor`))))))

(fn `ArrangeUIElements`
  (params (UIReferences :type "Array of /Game/Blueprints/BP_UserInterface Object Reference"))
  (locals (DefaultLocation :type "Vector Structure" :default (20.0 0.0 0.0)))
  (for (_array_element _array_index) UIReferences
    (`self.K2_SetActorTransform` _array_element (`KismetMathLibrary.MakeTransform` (+ (* (0.0 12.0 0.0) _array_index) (`local.DefaultLocation`)) (`self.K2_GetActorRotation` self) (`self.GetActorScale3D` _array_element)) false false)))

(fn `CalculateUIPlacement`
  (params (Actor :type "/Game/Blueprints/BP_Furniture_old Object Reference") (Index :type Integer))
  (returns (Location :type "Vector Structure") (Rotation :type "Rotator Structure") (Scale :type "Vector Structure"))
  (locals (TargetSize :type "Vector Structure" :default (10.0 10.0 10.0)) (DefaultLocation :type "Vector Structure" :default (0.0 12.0 0.0)))
  (return (+ (20.0 0.0 0.0) (* (`local.DefaultLocation`) Index)) (`SceneComponent.K2_GetComponentRotation` (`self.StaticMesh`)) (/ (`local.TargetSize`) (`.BoxExtent` (`self.GetActorBounds` Actor false)))))

(fn `FindOptions`
  (returns (Options :type "Array of /Game/Blueprints/BP_UserInterface Object Reference"))
  (bind _uieelements (`/Game/Blueprints/BP_Inventory.GetFurnitureUIElements` (`self.InventoryReference`) (`KismetArrayLibrary.Array_Get` (`self.Tags`) 1) 0))
  (bind _output_get (set `self.UIElements` _uieelements))
  (`self.ArrangeUIElements` _output_get)
  (return _output_get))

(fn `HasOptions`
  (returns (HasOptions :type Boolean))
  (return true))

(fn `InitializeAlternatives`)

(fn `IsSelectable`
  (returns (Selectable :type Boolean))
  (return true))

(fn `ReplaceActor`
  (bind _furnitureclass (`/Game/Blueprints/BP_Inventory.GetFurnitureClass` (`self.InventoryReference`) (`self.SelectedReference`)))
  (`|SpawnActorFromClass` _furnitureclass (`self.GetTransform` self) "AlwaysSpawn" "OverrideRootScale")
  (`self.K2_DestroyActor` self))

(fn `ReturnUIOptions`
  (bind _uielements (`self.UIElements`))
  (for _array_element _uielements
    (`self.K2_DetachFromActor` _array_element "KeepRelative" "KeepRelative" "KeepRelative")
    (`self.K2_SetActorLocation` _array_element (0.0 0.0 -200.0) false false))
  (`/Game/Blueprints/BP_Inventory.ReturnFurnitureUI` (`self.InventoryReference`) _uielements))

(fn `UpdateLocation`
  (if (`self.Selected`)
    (bind (_placementcenter _isvalidplacement _objectrotation) (`/Game/Blueprints/BP_ObjectController.GetPlacementResult` (`self.ObjController`)))
    (if _isvalidplacement
      (`SceneComponent.K2_SetWorldLocationAndRotation` (`self.DefaultSceneRoot`) (+ _placementcenter (`self.ObjectSelectedLocation`)) _objectrotation false false))))

(fn `UserConstructionScript`)