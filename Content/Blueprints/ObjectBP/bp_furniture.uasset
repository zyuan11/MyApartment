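; Furniture actor that tracks a selected state and supports hover highlighting.
; Its static mesh becomes visible when it begins overlapping an actor tagged "menu" and hidden when that overlap ends.
; Select and deselect functions toggle the selection flag.
; Hover functions set custom depth and stencil on the root's direct static mesh children, though ExitHover returns after clearing the first one.
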(event `self.ReceiveBeginPlay`
  (set `self.IsSelected` false))

(event `self.ReceiveActorBeginOverlap`
  (params (OtherActor :type "Actor Object Reference")))

(event `self.StaticMesh.OnComponentBeginOverlap`
  (params (OverlappedComponent :type "PrimitiveComponent Object Reference") (OtherActor :type "Actor Object Reference") (OtherComp :type "PrimitiveComponent Object Reference") (OtherBodyIndex :type Integer) (bFromSweep :type Boolean) (SweepResult :type "HitResult Structure (by ref)"))
  (if (`self.ActorHasTag` OtherActor "menu")
    (`SceneComponent.SetVisibility` (`self.StaticMesh`) true false)))

(event `self.StaticMesh.OnComponentEndOverlap`
  (params (OverlappedComponent :type "PrimitiveComponent Object Reference") (OtherActor :type "Actor Object Reference") (OtherComp :type "PrimitiveComponent Object Reference") (OtherBodyIndex :type Integer))
  (if (`self.ActorHasTag` OtherActor "menu")
    (`SceneComponent.SetVisibility` (`self.StaticMesh`) false false)))

(fn `DeselectFurniture`
  (set `self.IsSelected` false))

(fn `ExitHover`
  (for _array_element (`SceneComponent.GetChildrenComponents` (`self.DefaultSceneRoot`) false)
    (bind _asstatic_mesh_component (cast `StaticMeshComponent` _array_element))
    (`PrimitiveComponent.SetRenderCustomDepth` _asstatic_mesh_component false)
    (`PrimitiveComponent.SetCustomDepthStencilValue` _asstatic_mesh_component 0)
    (return)))

(fn `OnHover`
  (for _array_element (`SceneComponent.GetChildrenComponents` (`self.DefaultSceneRoot`) false)
    (bind _asstatic_mesh_component (cast `StaticMeshComponent` _array_element))
    (`PrimitiveComponent.SetRenderCustomDepth` _asstatic_mesh_component true)
    (`PrimitiveComponent.SetCustomDepthStencilValue` _asstatic_mesh_component 3)))

(fn `SelectFurniture`
  (set `self.IsSelected` true)
  (return))

(fn `UserConstructionScript`)