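; VR pawn for a Vive setup that sets a floor tracking origin and spawns a left menu controller and right object controller on its VR origin.
; The menu controller drives teleportation behind a camera fade to reduce nausea, capturing the destination during the fade delay and using a fixed height.
; Its menu button alternates shop transfers between TestShop and MainRoom.
; Object controller inputs forward selection, confirmation and face-button touch.
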(event `self.ReceiveBeginPlay`
  ;[1 1 1] Initialize HMD by attaching two controllers
  (`HeadMountedDisplayFunctionLibrary.SetTrackingOrigin` "Floor") ; Initialize Origin Location
  (`self.AttachControllers`))

(event `InputAction|MenuCtrlOpenMenu`
  (params (Key :type "Key Structure" :default "AnyKey"))
  ;[1 1 1] Menu Controller Input Events
  (:`Released`
    (`self.LoadShopLevel`)))

(event `InputAxis|MenuCtrlFaceBtnTouchY`
  (params (AxisValue :type "Float (single-precision)"))
  ;[1 1 1] Menu Controller Input Events
)

(event `InputAction|MenuCtrlTeleport`
  (params (Key :type "Key Structure" :default "AnyKey"))
  (bind _menucontroller (`self.MenuController`))
  ;[1 1 1] Menu Controller Input Events
  ;;[1 1 1] Handling Teleportation Input Event
  (:`Pressed`
    (`/Game/Blueprints/BP_MenuController.ActivateTeleport` _menucontroller))
  (:`Released`
    (`self.ExecuteTeleportation` _menucontroller)
    (`/Game/Blueprints/BP_MenuController.DisableTeleport` _menucontroller)))

(event `InputAxis|MenuCtrlFaceBtnTouchX`
  (params (AxisValue :type "Float (single-precision)"))
  ;[1 1 1] Menu Controller Input Events
)

(event `InputAction|MenuCtrlConfirmSelection`
  (params (Key :type "Key Structure" :default "AnyKey"))
  ;[1 1 1] Menu Controller Input Events
)

(event `InputAction|ObjectCtrlSelect`
  (params (Key :type "Key Structure" :default "AnyKey"))
  ;[1 0.295 0.295] Handing Selection
  (:`Released`
    (`/Game/Blueprints/BP_ObjectController.PressTrigger` (`self.ObjectController`))))

(event `InputAction|ObjectCtrlConfirmAlt`
  (params (Key :type "Key Structure" :default "AnyKey"))
  ;[1 0.295 0.295] Handling Layout Confirmation
  (:`Pressed`
    (`/Game/Blueprints/BP_ObjectController.ConfirmLayout` (`self.ObjectController`))))

(event `InputAction|ObjectCtrlAlternative`
  (params (Key :type "Key Structure" :default "AnyKey"))
  ;[1 1 1] Handling Object Alternative Options
)

(event `InputAxis|ObjectCtrlFaceBtnTouchX`
  (params (AxisValue :type "Float (single-precision)"))
  ;[1 1 1] Handling FaceButton Touch Event
  (`/Game/Blueprints/BP_ObjectController.ObjCtrlFaceBtnTouch` (`self.ObjectController`) AxisValue (stale `InputAxis|ObjectCtrlFaceBtnTouchY` AxisValue) :!label _label))

(event `InputAxis|ObjectCtrlFaceBtnTouchY`
  (params (AxisValue :type "Float (single-precision)"))
  ;[1 1 1] Handling FaceButton Touch Event
  (goto _label))

(event `InputAction|ObjectCtrlConfirmAlt`
  (params (Key :type "Key Structure" :default "AnyKey"))
  ;[1 1 1] Handling Object Alternative Options
  (:`Released`
    (`/Game/Blueprints/BP_ObjectController.ConfirmUI` (`self.ObjectController`))))

(event `ExecuteTeleportation`
  (params (MenuController :type "/Game/Blueprints/BP_MenuController Object Reference"))
  (bind _returnvalue (`GameplayStatics.GetPlayerCameraManager` 0))
  ;[1 1 1] Execute Teleportation
  ;;[1 1 1] Validate teleportation condition satisified
  (if (`self.IsTeleporting`)
    _
    (elif (`/Game/Blueprints/BP_MenuController.ValidTeleportPoint` MenuController)
      (`|ExecutionSequence`
        (:`then_0`
          ;;[1 1 1] Camera fade while teleporting to reduce nausea effect
          (set `self.IsTeleporting` true)
          (`PlayerCameraManager.StartCameraFade` :`self` _returnvalue :`ToAlpha` 1.0 :`Duration` (`self.FadeOutDuration`) :`bHoldWhenFinished` true)
          (`KismetSystemLibrary.Delay` (`self.FadeOutDuration`))
          (`/Game/Blueprints/BP_MenuController.DisableTeleport` MenuController)
          (`self.K2_TeleportTo` (`KismetMathLibrary.MakeVector` (.x (stale _location)) (.y (stale _location)) 50.0))
          (`PlayerCameraManager.StartCameraFade` :`self` _returnvalue :`FromAlpha` 1.0 :`Duration` (`self.FadeOutDuration`))
          (set `self.IsTeleporting` false))
        (:`then_1`
          (bind _location (`/Game/Blueprints/BP_MenuController.GetTeleportLocation` MenuController))))
      (else
        (`/Game/Blueprints/BP_MenuController.DisableTeleport` MenuController)))))

(fn `AttachControllers`
  (locals (DefaultTransform :type "Transform Structure"))
  (bind _defaulttransform (`local.DefaultTransform`))
  (`|ExecutionSequence`
    (:`then_0`
      ;[1 1 1] Attach Left Controller
      (bind _returnvalue (`|SpawnActorFromClass` "/Game/Blueprints/BP_MenuController.BP_MenuController_C" _defaulttransform "AlwaysSpawn" "OverrideRootScale" self "Left"))
      (set `self.MenuController` _returnvalue)
      (`self.K2_AttachToComponent` _returnvalue (`self.VROrigin`) "None" "SnapToTarget" "SnapToTarget" "KeepWorld" false))
    (:`then_1`
      ;[1 1 1] Attach Right Controller
      (bind _returnvalue_2 (`|SpawnActorFromClass` "/Game/Blueprints/BP_ObjectController.BP_ObjectController_C" _defaulttransform "AlwaysSpawn" "OverrideRootScale" self "Right"))
      (set `self.ObjectController` _returnvalue_2)
      (`self.K2_AttachToComponent` _returnvalue_2 (`self.VROrigin`) "None" "SnapToTarget" "SnapToTarget" "KeepWorld" false))))

(fn `LoadShopLevel`
  (if (`self.NewVar_0`)
    (`self.TransferShop` "TestShop")
    (else
      (`self.TransferShop` "MainRoom")))
  (set `self.NewVar_0` (not (`self.NewVar_0`))))

(fn `UserConstructionScript`)