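; Drawing board on which the user draws an apartment wall layout that then becomes raised 3D walls.
; Wall segments follow the hit point in four directions, sized in 16-unit steps with length labels, and flag when the outline returns to its origin.
; Confirmed segments are mirrored to Bp_ground.
; After layout confirmation, Tick rotates the board, scales the walls up to target height, then has the ground relocate the user to the apartment.
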(event `self.ReceiveBeginPlay`
  (bind _outactors (`GameplayStatics.GetAllActorsOfClass` "/Game/Blueprints/AptBP/bp_ground.bp_ground_C"))
  (set `self.ground` (`KismetArrayLibrary.Array_Get` _outactors)))

(event `self.ReceiveTick`
  (params (DeltaSeconds :type "Float (single-precision)"))
  (if (`self.IsReadyToRaiseWall`)
    (`self.RaiseWall` DeltaSeconds)
    (elif (`self.LayoutConfirmed`)
      (`self.PushBoard` DeltaSeconds))))

(fn `BuildNewWall`
  (bind _lastcomfirmpointloc (`self.LastComfirmPointLoc`))
  (bind _returnvalue (`|SpawnActorFromClass` "/Game/Blueprints/UserInputBP/bp_wall.bp_wall_C" (`KismetMathLibrary.Conv_VectorToTransform` _lastcomfirmpointloc) "Undefined" "OverrideRootScale"))
  (`self.K2_AttachToActor` _returnvalue self "None" "KeepWorld" "KeepWorld" "KeepWorld" true)
  (bind _output_get (set `self.currWall` _returnvalue))
  (`/Game/Blueprints/UserInputBP/bp_wall.SetOriginalLoc` _output_get _lastcomfirmpointloc)
  (return))

(fn `CalculateEndingLocOfWall`
  (returns (EndingLoc_o :type "Vector Structure"))
  (locals (result :type "Vector Structure"))
  (bind _currwall (`self.currWall`))
  (bind (_lastcomfirmpointloc_x _lastcomfirmpointloc_y _lastcomfirmpointloc_z) (`KismetMathLibrary.BreakVector` (`self.LastComfirmPointLoc`)))
  (bind (_lastcomfirmpointloc_x_2 _lastcomfirmpointloc_y_2 _lastcomfirmpointloc_z_2) (`KismetMathLibrary.BreakVector` (`self.LastComfirmPointLoc`)))
  (bind (_lastcomfirmpointloc_x_3 _lastcomfirmpointloc_y_3 _lastcomfirmpointloc_z_3) (`KismetMathLibrary.BreakVector` (`self.LastComfirmPointLoc`)))
  (bind (_lastcomfirmpointloc_x_4 _lastcomfirmpointloc_y_4 _lastcomfirmpointloc_z_4) (`KismetMathLibrary.BreakVector` (`self.LastComfirmPointLoc`)))
  (bind (_returnvalue_x _returnvalue_y) (`KismetMathLibrary.BreakVector` (`self.K2_GetActorLocation` _currwall)))
  (bind (_returnvalue_x_2 _returnvalue_y_2 _returnvalue_z) (`KismetMathLibrary.BreakVector` (`self.K2_GetActorLocation` _currwall)))
  (switch `int` (`self.CurrDir`)
    (:`0`
      (set `local.result` (`KismetMathLibrary.MakeVector` _lastcomfirmpointloc_x_2 _lastcomfirmpointloc_y_2 (+ (* (- _returnvalue_z _lastcomfirmpointloc_z_2) 2.0) _lastcomfirmpointloc_z_2))))
    (:`1`
      (set `local.result` (`KismetMathLibrary.MakeVector` _lastcomfirmpointloc_x_3 _lastcomfirmpointloc_y_3 (- _lastcomfirmpointloc_z_3 (* (- _lastcomfirmpointloc_z_3 _returnvalue_z) 2.0)))))
    (:`2`
      (set `local.result` (`KismetMathLibrary.MakeVector` _lastcomfirmpointloc_x_4 (- _lastcomfirmpointloc_y_4 (* (- _lastcomfirmpointloc_y_4 _returnvalue_y) 2.0)) _lastcomfirmpointloc_z_4)))
    (:`3`
      (set `local.result` (`KismetMathLibrary.MakeVector` _lastcomfirmpointloc_x (+ (* (- _returnvalue_y _lastcomfirmpointloc_y) 2.0) _lastcomfirmpointloc_y) _lastcomfirmpointloc_z))))
  (return (`local.result`)))

(fn `ConfirmCurrWall`
  (bind _currdir (`self.CurrDir`))
  (bind _currwalllength (`self.CurrWallLength`))
  (bind _ground (`self.ground`))
  (`KismetArrayLibrary.Array_Add` (`self.Dirs`) _currdir)
  (`KismetArrayLibrary.Array_Add` (`self.Lengths`) _currwalllength)
  (`KismetArrayLibrary.Array_Add` (`self.Walls`) (`self.currWall`))
  (bind _endingloc_o (`self.CalculateEndingLocOfWall`))
  (`/Game/Blueprints/AptBP/bp_ground.BuildWall` (`self.ground`) _currdir _currwalllength)
  (if (== _endingloc_o (`self.OriginalLoc`) :`ErrorTolerance` 1.0)
    (set `self.IsBackToOrigin` true)
    (else
      (`self.SetLastComfirmPointLoc` _endingloc_o)
      (bind _groundloc (`/Game/Blueprints/AptBP/bp_ground.DrawingBoardToGroundLoc` _ground _endingloc_o))
      (`/Game/Blueprints/AptBP/bp_ground.SetLastConfimedLoc` _ground _groundloc)))
  (return))

(fn `ConfirmLayout`
  (set `self.LayoutConfirmed` true)
  (return))

(fn `GoUp_Down_Left_Right`
  (locals (y :type "Float (double-precision)") (z :type "Float (double-precision)") (dir_o :type Integer :default -1))
  (bind (_hitloc_x _hitloc_y _hitloc_z) (`KismetMathLibrary.BreakVector` (`self.HitLoc`)))
  (bind (_lastcomfirmpointloc_x _lastcomfirmpointloc_y _lastcomfirmpointloc_z) (`KismetMathLibrary.BreakVector` (`self.LastComfirmPointLoc`)))
  (set `local.y` (- _hitloc_y _lastcomfirmpointloc_y))
  (set `local.z` (- _hitloc_z _lastcomfirmpointloc_z))
  (if (> (`local.y`) 0.0)
    ;[0.5015 0.9099 1] check if go left
    (if (and (> (`local.z`) (- 0.0 (`local.y`))) (<= (`local.z`) (`local.y`)))
      (set `self.CurrDir` 3)
      (else
        ;[0.5015 0.9099 1] check if go up
        (if (> (`local.z`) (`local.y`))
          (set `self.CurrDir` 0)
          (else
            ;[0.5015 0.9099 1] check if go down
            (if (<= (`local.z`) (- 0.0 (`local.y`)))
              (set `self.CurrDir` 1))))))
    (else
      ;[0.5015 0.9099 1] check if go right
      (if (and (< (`local.z`) (- 0.0 (`local.y`))) (>= (`local.z`) (`local.y`)))
        (set `self.CurrDir` 2)
        (else
          ;[0.5015 0.9099 1] check if go up
          (if (>= (`local.z`) (- 0.0 (`local.y`)))
            (set `self.CurrDir` 0)
            (else
              ;[0.5015 0.9099 1] check if go down
              (if (< (`local.z`) (`local.y`)) :!pinned true
                (set `self.CurrDir` 1))))))))
  (return) ; 0 for up, 1 for down, 2 for left, 3 for right
)

(fn `PushBoard`
  (params (DeltaTime :type "Float (double-precision)"))
  (if (== (`self.K2_GetActorRotation`) (struct :`Pitch` 90.0) :`ErrorTolerance` 1.0)
    (set `self.IsReadyToRaiseWall` true)
    (set `self.LayoutConfirmed` false)
    (else
      (`self.K2_AddActorLocalRotation` (`KismetMathLibrary.MakeRotator` 0.0 (* DeltaTime (`self.RotationSpeed`))))))
  (return))

(fn `RaiseWall`
  (params (DeltaTime :type "Float (double-precision)"))
  (bind _walls (`self.Walls`))
  (for (_array_element _array_index) _walls
    (bind _cube (`/Game/Blueprints/UserInputBP/bp_wall.cube` _array_element))
    (bind (_returnvalue_x _returnvalue_y _returnvalue_z) (`KismetMathLibrary.BreakVector` (`SceneComponent.K2_GetComponentScale` _cube)))
    (if (`KismetMathLibrary.NearlyEqual_FloatFloat` _returnvalue_z (* (`KismetMathLibrary.Conv_IntToDouble` (`self.TargetWallHeight`)) 16.0 0.01) 0.1)
      (if (== (+ _array_index 1) (`KismetArrayLibrary.Array_Length` _walls))
        (set `self.IsReadyToRaiseWall` false)
        (`/Game/Blueprints/AptBP/bp_ground.LocateUserToApt` (`self.ground`))
        (set `self.WallRaised` false)
        (set `self.IsReadyToRaiseWall` false)
        (set `self.LayoutConfirmed` false))
      (else
        (`SceneComponent.SetWorldScale3D` _cube (`KismetMathLibrary.MakeVector` _returnvalue_x _returnvalue_y (+ _returnvalue_z (* (`self.RaiseSpeed`) DeltaTime))))))))

(fn `SetHitLoc`
  (params (HitLoc_i :type "Vector Structure"))
  (returns (HitLoc_o :type "Vector Structure"))
  (bind _output_get (set `self.HitLoc` (`KismetMathLibrary.MakeVector` (- HitLoc_i_X -10.0) HitLoc_i_Y HitLoc_i_Z)))
  (return _output_get))

(fn `SetLastComfirmPointLoc`
  (params (LastComfirmPointLoc_i :type "Vector Structure"))
  (set `self.LastComfirmPointLoc` LastComfirmPointLoc_i)
  (return))

(fn `SetOriginalLoc`
  (params (OriginalLoc_i :type "Vector Structure"))
  (set `self.OriginalLoc` OriginalLoc_i)
  (return))

(fn `StartDrawingMode`
  (params (HitLoc :type "Vector Structure"))
  (`self.SetLastComfirmPointLoc` HitLoc)
  (`self.SetOriginalLoc` HitLoc)
  (`/Game/Blueprints/AptBP/bp_ground.SetOriginalLoc` (`self.ground`) HitLoc)
  (return))

(fn `UpdateCurrBuildingWall`
  (`self.GoUp_Down_Left_Right`)
  (switch `int` (`self.CurrDir`)
    (:`Default`
      _)
    (:`0`
      (`self.UpdateWallsInUpDir`))
    (:`1`
      (`self.UpdateWallsInDownDir`))
    (:`2`
      (`self.UpdateWallsInRightDir`))
    (:`3`
      (`self.UpdateWallsInLeftDir`)))
  (return))

(fn `UserConstructionScript`)