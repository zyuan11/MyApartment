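; BP_UserInterface is an actor Blueprint that highlights its meshes on hover and provides stub queries for options and selection.
; OnHover enables custom depth and sets a stencil value on static mesh components directly under the scene root; ExitHover reverses both.
; HasOptions and IsSelectable always return false, and FindOptions holds no logic of its own.
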(event `/Game/Blueprints/BP_ObjectInterface.OnHover`
  ;[1 1 1] OnHover Implementation
  (for _array_element (`SceneComponent.GetChildrenComponents` (`self.DefaultSceneRoot`) false)
    (bind _asstatic_mesh_component (cast `StaticMeshComponent` _array_element))
    (`PrimitiveComponent.SetRenderCustomDepth` _asstatic_mesh_component true)
    (`PrimitiveComponent.SetCustomDepthStencilValue` _asstatic_mesh_component 3)))

(event `/Game/Blueprints/BP_ObjectInterface.ExitHover`
  ;[1 1 1] ExitHover Implementation
  (for _array_element (`SceneComponent.GetChildrenComponents` (`self.DefaultSceneRoot`) false)
    (bind _asstatic_mesh_component (cast `StaticMeshComponent` _array_element))
    (`PrimitiveComponent.SetRenderCustomDepth` _asstatic_mesh_component false)
    (`PrimitiveComponent.SetCustomDepthStencilValue` _asstatic_mesh_component 0)))

(fn `FindOptions`
  (returns (Options :type "Array of /Game/Blueprints/BP_UserInterface Object Reference"))
  (return (`|MakeArray` null :!type "/Game/Blueprints/BP_UserInterface Object Reference")))

(fn `HasOptions`
  (returns (HasOptions :type Boolean))
  (return false))

(fn `IsSelectable`
  (returns (Selectable :type Boolean))
  (return false))

(fn `UserConstructionScript`)