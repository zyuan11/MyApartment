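; Floating menu actor for picking placeable floor, ceiling and wall objects, opened in front of the camera at its yaw.
; On BeginPlay it gathers "ForMenu"-tagged actors, scales them down, attaches them hidden and sorts them by type.
; Opening lays floor and ceiling objects on eight placeholders; wall layout is an empty stub.
; Controller distance scrolls the pages by offsetting meshes; half-page snap logic exists but is disconnected.
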(event `self.ReceiveBeginPlay`
  (`SceneComponent.SetVisibility` (`self.menu_background`) false false)
  (`self.K2_SetActorLocation` (0.0 0.0 0.0))
  (set `self.IsOpen` false)
  (set `self.PgCnt` 0)
  (`self.SetObjsLocOnMenu`)
  (`self.MenuContentInit`)
  (`self.MenuSwitchReset` 0))

(event `self.ReceiveTick`
  (params (DeltaSeconds :type "Float (single-precision)"))
  (if (`self.IsOpen`)
    _))

(fn `CellingObjLocSet`
  (params (Obj :type "/Game/Blueprints/ObjectBP/bp_cellingobject Object Reference") (Ind :type Integer))
  (bind _staticmesh (`/Game/Blueprints/ObjectBP/bp_furniture.StaticMesh` Obj))
  (bind (_returnvalue_x _returnvalue_y _returnvalue_z) (`KismetMathLibrary.BreakVector` (`SceneComponent.K2_GetComponentScale` _staticmesh)))
  (bind (_returnvalue_x_2 _returnvalue_y_2 _returnvalue_z_2) (`KismetMathLibrary.BreakVector` (`SceneComponent.K2_GetComponentLocation` (`KismetArrayLibrary.Array_Get` (`self.MenuPlaceHolders`) Ind))))
  (if (<= Ind 7)
    (`SceneComponent.K2_SetWorldLocation` _staticmesh (`KismetMathLibrary.MakeVector` _returnvalue_x_2 (+ _returnvalue_y_2 120.0) (+ _returnvalue_z_2 (* 0.5 100.0 _returnvalue_z))) false false))
  (return))

(fn `CheckIfReachDest`
  (bind _pgcnt (`self.PgCnt`))
  (`self.IsMovingHori`
    (:`SetToLeft`
      (`/Engine/EditorBlueprintResources/StandardMacros.IncrementInt` _pgcnt
        (:`  `
          _)))
    (:`SetToRight`
      (`/Engine/EditorBlueprintResources/StandardMacros.DecrementInt` _pgcnt
        (:`  `
          _)))
    (:`ResetBackToLeft`
      _)
    (:`ResetBackToRight`
      _))
  (switch `int` (`self.PgCnt`)
    (:`0`
      (`self.FloorObjLocSet` (`KismetMathLibrary.MakeVector` 0.0 (`self.DistToMove_SwitchChk`))))))

(fn `CloseMenu`
  (set `self.IsOpen` false)
  (`SceneComponent.SetVisibility` (`self.menu_background`) false false)
  (for _array_element (`self.FloorObjs`)
    (`SceneComponent.SetVisibility` (`/Game/Blueprints/ObjectBP/bp_furniture.StaticMesh` _array_element) false false))
  (for _array_element_2 (`self.CellingObjs`)
    (`SceneComponent.SetVisibility` (`/Game/Blueprints/ObjectBP/bp_furniture.StaticMesh` _array_element_2) false false))
  (for _array_element_3 (`self.WallObjs`)
    (`SceneComponent.SetVisibility` (`/Game/Blueprints/ObjectBP/bp_furniture.StaticMesh` _array_element_3) false false))
  (return))

(fn `FloorObjLocSet`
  (params (OffsetToAdd :type "Vector Structure"))
  (locals (distToMove :type "Float (double-precision)"))
  (for _array_element (`self.FloorObjs`)
    (`SceneComponent.K2_AddLocalOffset` (`/Game/Blueprints/ObjectBP/bp_furniture.StaticMesh` _array_element) OffsetToAdd false true))
  (return))

(fn `MenuContentInit`
  (bind _outactors (`GameplayStatics.GetAllActorsWithTag` "ForMenu"))
  (for _array_element _outactors
    ;[0.6784 0.9922 1] CellingObjs
    (bind _asbp_cellingobject (cast `/Game/Blueprints/ObjectBP/bp_cellingobject` _array_element)
      (:`then`
        (bind _objscaleformenu (`self.RescaleObjForMenu` (`/Game/Blueprints/ObjectBP/bp_furniture.ObjScale` _asbp_cellingobject) (`self.GetActorScale3D` _asbp_cellingobject)))
        (`self.SetActorScale3D` _asbp_cellingobject _objscaleformenu)
        (set `/Game/Blueprints/ObjectBP/bp_furniture.InMenu` true _asbp_cellingobject)
        (`self.K2_AttachToComponent` _asbp_cellingobject (`self.DefaultSceneRoot`) "None" "KeepRelative" "KeepWorld" "KeepRelative" true)
        (`SceneComponent.SetVisibility` (`/Game/Blueprints/ObjectBP/bp_furniture.StaticMesh` _asbp_cellingobject) false false)
        (bind _returnvalue (`KismetArrayLibrary.Array_Add` (`self.CellingObjs`) _asbp_cellingobject))
        (`self.CellingObjLocSet` _asbp_cellingobject _returnvalue))
      (:`CastFailed`
        ;[0.6784 0.9922 1] WallObjs
        (bind _asbp_wallobject (cast `/Game/Blueprints/ObjectBP/bp_wallobject` _array_element)
          (:`then`
            (bind _objscaleformenu_2 (`self.RescaleObjForMenu` (`/Game/Blueprints/ObjectBP/bp_furniture.ObjScale` _asbp_wallobject) (`self.GetActorScale3D` _asbp_wallobject)))
            (`self.SetActorScale3D` _asbp_wallobject _objscaleformenu_2)
            (set `/Game/Blueprints/ObjectBP/bp_furniture.InMenu` true _asbp_wallobject)
            (`self.K2_AttachToComponent` _asbp_wallobject (`self.DefaultSceneRoot`) "None" "KeepRelative" "KeepWorld" "KeepRelative" true)
            (`SceneComponent.SetVisibility` (`/Game/Blueprints/ObjectBP/bp_furniture.StaticMesh` _asbp_wallobject) false false)
            (`KismetArrayLibrary.Array_Add` (`self.WallObjs`) _asbp_wallobject))
          (:`CastFailed`
            ;[0.6784 0.9922 1] FloorObjs
            (bind _asbp_floorobject (cast `/Game/Blueprints/ObjectBP/bp_floorobject` _array_element))
            (bind _objscaleformenu_3 (`self.RescaleObjForMenu` (`/Game/Blueprints/ObjectBP/bp_furniture.ObjScale` _asbp_floorobject) (`self.GetActorScale3D` _asbp_floorobject)))
            (`self.SetActorScale3D` _asbp_floorobject _objscaleformenu_3)
            (set `/Game/Blueprints/ObjectBP/bp_furniture.InMenu` true _asbp_floorobject)
            (`self.K2_AttachToComponent` _asbp_floorobject (`self.DefaultSceneRoot`) "None" "KeepRelative" "KeepWorld" "KeepRelative" true)
            (`SceneComponent.SetVisibility` (`/Game/Blueprints/ObjectBP/bp_furniture.StaticMesh` _asbp_floorobject) false false)
            (`KismetArrayLibrary.Array_Add` (`self.FloorObjs`) _asbp_floorobject))))))
  (return))

(fn `MenuSwitch_Left`
  (params (ControllerMovingDist :type "Float (double-precision)"))
  (locals (MovingDist_i :type "Float (double-precision)"))
  (bind _returnvalue (- 0.0 (`local.MovingDist_i`)))
  (bind _output_get (set `local.MovingDist_i` (* ControllerMovingDist 5.0)))
  (set `self.MenuMovingDist` (+ _output_get (`self.MenuMovingDist`)))
  (switch `int` (`self.PgCnt`)
    (:`Default`
      _)
    (:`0`
      (for _array_element (`self.FloorObjs`)
        (`SceneComponent.K2_AddLocalOffset` (`/Game/Blueprints/ObjectBP/bp_furniture.StaticMesh` _array_element) (`KismetMathLibrary.MakeVector` 0.0 _returnvalue) false false))
      (for _array_element_2 (`self.CellingObjs`)
        (`SceneComponent.K2_AddLocalOffset` (`/Game/Blueprints/ObjectBP/bp_furniture.StaticMesh` _array_element_2) (`KismetMathLibrary.MakeVector` 0.0 _returnvalue) false false)))
    (:`1`
      (for _array_element_3 (`self.CellingObjs`)
        (`SceneComponent.K2_AddLocalOffset` (`/Game/Blueprints/ObjectBP/bp_furniture.StaticMesh` _array_element_3) (`KismetMathLibrary.MakeVector` 0.0 _returnvalue) false false))
      (for _array_element_4 (`self.WallObjs`)
        (`SceneComponent.K2_AddWorldOffset` (`/Game/Blueprints/ObjectBP/bp_furniture.StaticMesh` _array_element_4) (`KismetMathLibrary.MakeVector` 0.0 _returnvalue) false false)))
    (:`2`
      _))
  (return))

(fn `MenuSwitch_Right`
  (params (ControllerMovingDist :type "Float (double-precision)"))
  (locals (MovingDist_i :type "Float (double-precision)"))
  (bind _movingdist_i (`local.MovingDist_i`))
  (bind _output_get (set `local.MovingDist_i` (* ControllerMovingDist 5.0)))
  (set `self.MenuMovingDist` (+ _output_get (`self.MenuMovingDist`)))
  (switch `int` (`self.PgCnt`)
    (:`Default`
      _)
    (:`0`
      _)
    (:`1`
      (for _array_element (`self.FloorObjs`)
        (`SceneComponent.K2_AddLocalOffset` (`/Game/Blueprints/ObjectBP/bp_furniture.StaticMesh` _array_element) (`KismetMathLibrary.MakeVector` 0.0 _movingdist_i) false false))
      (for _array_element_2 (`self.CellingObjs`)
        (`SceneComponent.K2_AddLocalOffset` (`/Game/Blueprints/ObjectBP/bp_furniture.StaticMesh` _array_element_2) (`KismetMathLibrary.MakeVector` 0.0 _movingdist_i) false false)))
    (:`2`
      (for _array_element_3 (`self.CellingObjs`)
        (`SceneComponent.K2_AddLocalOffset` (`/Game/Blueprints/ObjectBP/bp_furniture.StaticMesh` _array_element_3) (`KismetMathLibrary.MakeVector` 0.0 _movingdist_i) false false))
      (for _array_element_4 (`self.WallObjs`)
        (`SceneComponent.K2_AddWorldOffset` (`/Game/Blueprints/ObjectBP/bp_furniture.StaticMesh` _array_element_4) (`KismetMathLibrary.MakeVector` 0.0 _movingdist_i) false false))))
  (return))

(fn `MenuSwitchReset`
  (params (SwitchDir :type Integer))
  (set `self.SwitchDir` SwitchDir)
  (set `self.MenuMovingDist` 0.0)
  (return))

(fn `MenuSwitchVertical`
  (params (ControllerMovingDist :type "Float (double-precision)") (MovingDir :type Boolean))
  (locals (MovingDist_i :type "Float (double-precision)") (MovingDist_Dir :type "Float (double-precision)"))
  (bind _movingdist_dir (`local.MovingDist_Dir`))
  (bind _output_get (set `local.MovingDist_i` (* ControllerMovingDist 5.0)))
  (set `self.MenuMovingDist` (+ _output_get (`self.MenuMovingDist`)))
  (if MovingDir
    (set `local.MovingDist_Dir` (`local.MovingDist_i`))
    (else
      (set `local.MovingDist_Dir` (- 0.0 (`local.MovingDist_i`)))))
  (switch `int` (`self.PgCnt`)
    (:`Default`
      _)
    (:`0`
      (for _array_element (`self.FloorObjs`)
        (`SceneComponent.K2_AddLocalOffset` (`/Game/Blueprints/ObjectBP/bp_furniture.StaticMesh` _array_element) (`KismetMathLibrary.MakeVector` 0.0 0.0 _movingdist_dir) false false)))
    (:`1`
      (for _array_element_2 (`self.CellingObjs`)
        (`SceneComponent.K2_AddLocalOffset` (`/Game/Blueprints/ObjectBP/bp_furniture.StaticMesh` _array_element_2) (`KismetMathLibrary.MakeVector` 0.0 0.0 _movingdist_dir) false false)))
    (:`2`
      (for _array_element_3 (`self.WallObjs`)
        (`SceneComponent.K2_AddLocalOffset` (`/Game/Blueprints/ObjectBP/bp_furniture.StaticMesh` _array_element_3) (`KismetMathLibrary.MakeVector` 0.0 0.0 _movingdist_dir) false false))))
  (return))

(fn `OpenMenu`
  (params (cameraLoc :type "Vector Structure") (cameraRot :type "Rotator Structure"))
  (locals (CamLoc :type "Vector Structure") (CamRot :type "Rotator Structure"))
  (bind (_camloc_x _camloc_y _camloc_z) (`KismetMathLibrary.BreakVector` (`local.CamLoc`)))
  (bind _defaultsceneroot (`self.DefaultSceneRoot`))
  (bind (_camrot_roll _camrot_pitch _camrot_yaw) (`KismetMathLibrary.BreakRotator` (`local.CamRot`)))
  (set `local.CamLoc` cameraLoc)
  (bind _output_get (set `local.CamRot` cameraRot))
  (`SceneComponent.K2_SetWorldLocation` _defaultsceneroot (`KismetMathLibrary.MakeVector` (+ (* (`KismetMathLibrary.DegCos` (.yaw _output_get)) 70.0) _camloc_x) (+ (* (`KismetMathLibrary.DegCos` (- 90.0 (.yaw _output_get))) 70.0) _camloc_y) _camloc_z) false false)
  (`SceneComponent.K2_SetWorldRotation` _defaultsceneroot (`KismetMathLibrary.MakeRotator` 0.0 0.0 _camrot_yaw) false false)
  (set `self.IsOpen` true)
  (`SceneComponent.SetVisibility` (`self.menu_background`) true false)
  (`self.ResetMenuContent`)
  (return))

(fn `RemoveFromCellingObjs`
  (params (ObjToRemove :type "/Game/Blueprints/ObjectBP/bp_cellingobject Object Reference"))
  (`KismetArrayLibrary.Array_RemoveItem` (`self.CellingObjs`) ObjToRemove)
  (return))

(fn `RemoveFromFloorObjs`
  (params (ObjToRemove :type "/Game/Blueprints/ObjectBP/bp_floorobject Object Reference"))
  ;[0.3647 0.251 0.298] remove placed obj from menu
  (`KismetArrayLibrary.Array_RemoveItem` (`self.FloorObjs`) ObjToRemove)
  (return))

(fn `RescaleObjForMenu`
  (params (ObjScale :type "Float (double-precision)") (NewParam :type "Vector Structure"))
  (returns (ObjScaleForMenu :type "Vector Structure"))
  (return (* NewParam (/ 0.2 ObjScale))))

(fn `ResetCellingObjs`
  (for (_array_element _array_index) (`self.CellingObjs`)
    (`self.CellingObjLocSet` _array_element _array_index)
    (`SceneComponent.SetVisibility` (`/Game/Blueprints/ObjectBP/bp_furniture.StaticMesh` _array_element) true false))
  (return))

(fn `ResetFloorObjs`
  (for (_array_element _array_index) (`self.FloorObjs`)
    (if (<= _array_index 7)
      (bind _staticmesh (`/Game/Blueprints/ObjectBP/bp_furniture.StaticMesh` _array_element))
      (bind (_returnvalue_x _returnvalue_y _returnvalue_z) (`KismetMathLibrary.BreakVector` (`SceneComponent.K2_GetComponentLocation` (`KismetArrayLibrary.Array_Get` (`self.MenuPlaceHolders`) _array_index))))
      (bind (_returnvalue_x_2 _returnvalue_y_2 _returnvalue_z_2) (`KismetMathLibrary.BreakVector` (`SceneComponent.K2_GetComponentScale` _staticmesh)))
      (`SceneComponent.K2_SetWorldLocation` _staticmesh (`KismetMathLibrary.MakeVector` _returnvalue_x _returnvalue_y (- _returnvalue_z (* 0.5 100.0 _returnvalue_z_2))) false false)
      (`SceneComponent.SetVisibility` _staticmesh true false)))
  (return))

(fn `ResetMenuContent`
  (set `self.PgCnt` 0)
  (`self.ResetFloorObjs`)
  (`self.ResetCellingObjs`)
  (`self.ResetWallObjs`)
  (return))

(fn `ResetWallObjs`)

(fn `SetObjsLocOnMenu`
  (bind _menuplaceholders (`self.MenuPlaceHolders`))
  (`|ExecutionSequence`
    (:`then_0`
      (`KismetArrayLibrary.Array_Add` _menuplaceholders (`self.Obj1Loc`)))
    (:`then_1`
      (`KismetArrayLibrary.Array_Add` _menuplaceholders (`self.Obj2Loc`)))
    (:`then_2`
      (`KismetArrayLibrary.Array_Add` _menuplaceholders (`self.Obj3Loc`)))
    (:`then_3`
      (`KismetArrayLibrary.Array_Add` _menuplaceholders (`self.Obj4Loc`)))
    (:`then_4`
      (`KismetArrayLibrary.Array_Add` _menuplaceholders (`self.Obj5Loc`)))
    (:`then_5`
      (`KismetArrayLibrary.Array_Add` _menuplaceholders (`self.Obj6Loc`)))
    (:`then_6`
      (`KismetArrayLibrary.Array_Add` _menuplaceholders (`self.Obj7Loc`)))
    (:`then_7`
      (`KismetArrayLibrary.Array_Add` _menuplaceholders (`self.Obj8Loc`))
      (return))))

(fn `UserConstructionScript`)