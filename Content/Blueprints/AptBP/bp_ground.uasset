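; Ground actor for a VR apartment builder that turns points from a drawing board into full-size walls.
; Drawing-board coordinates are remapped and scaled onto the ground to set the origin and last confirmed point.
; BuildWall offsets half the given length from that point in one of four directions, then spawns, scales and attaches a Bp_RealWall, storing it in Walls.
; It also caches the Vive pawn and can teleport it to the world origin.
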(event `self.ReceiveBeginPlay`
  (bind _outactors (`GameplayStatics.GetAllActorsOfClass` "/Game/Blueprints/BP_VivePawn.BP_VivePawn_C"))
  (set `self.user` (`KismetArrayLibrary.Array_Get` _outactors)))

(event `self.ReceiveTick`
  (params (DeltaSeconds :type "Float (single-precision)")))

(fn `BuildWall`
  (params (dir_i :type Integer) (length_i :type Integer))
  (locals (WallLoc :type "Vector Structure") (localWallScale :type "Vector Structure"))
  (switch `int` dir_i
    (:`0`
      (bind (_wallloc _wallscale) (`self.UpWallCalculation` length_i)
        (:`return`
          (set `local.WallLoc` _wallloc)
          (set `local.localWallScale` _wallscale))))
    (:`1`
      (bind (_wallloc_2 _wallscale_2) (`self.DownWallCalculation` length_i)
        (:`return`
          (set `local.WallLoc` _wallloc_2)
          (set `local.localWallScale` _wallscale_2))))
    (:`2`
      (bind (_wallloc_3 _wallscale_3) (`self.RightWallCalculation` length_i)
        (:`return`
          (set `local.WallLoc` _wallloc_3)
          (set `local.localWallScale` _wallscale_3))))
    (:`3`
      (bind (_wallloc_4 _wallscale_4) (`self.LeftWallCalculation` length_i)
        (:`return`
          (set `local.WallLoc` _wallloc_4)
          (set `local.localWallScale` _wallscale_4)))))
  (bind _returnvalue (`|SpawnActorFromClass` "/Game/Blueprints/AptBP/bp_RealWall.bp_RealWall_C" (`KismetMathLibrary.Conv_VectorToTransform` (`local.WallLoc`)) "AlwaysSpawn" "OverrideRootScale"))
  (`self.K2_AttachToActor` _returnvalue self "None" "KeepWorld" "KeepWorld" "KeepWorld" true)
  (`SceneComponent.SetRelativeScale3D` (`/Game/Blueprints/AptBP/bp_RealWall.Cube` _returnvalue) (`local.localWallScale`))
  (`KismetArrayLibrary.Array_Add` (`self.Walls`) _returnvalue)
  (return))

(fn `CalculateBuildingWallLoc`
  (params (Dir_i :type Integer) (length_i :type Integer)))

(fn `DrawingBoardToGroundLoc`
  (params (DrawingBoardLoc_i :type "Vector Structure"))
  (returns (GroundLoc :type "Vector Structure"))
  (return (`KismetMathLibrary.MakeVector` (* (- DrawingBoardLoc_i_Z 525.0) -6.25) (* DrawingBoardLoc_i_Y 6.25) 175.0)))

(fn `LocateUserToApt`
  (`self.K2_SetActorLocation` (`self.user`) (0.0 0.0 0.0) false true)
  (return))

(fn `SetLastConfimedLoc`
  (params (LastConfirmedLoc_i :type "Vector Structure"))
  (set `self.LastConfirmedPointLoc` LastConfirmedLoc_i)
  (return))

(fn `SetOriginalLoc`
  (params (OriginalLocOfDrawingBoard :type "Vector Structure"))
  (bind _groundloc (`self.DrawingBoardToGroundLoc` OriginalLocOfDrawingBoard))
  (bind _output_get (set `self.OriginalLoc` _groundloc))
  (`self.SetLastConfimedLoc` _output_get)
  (return))

(fn `UserConstructionScript`)