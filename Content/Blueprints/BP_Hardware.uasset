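; BP_Hardware is a non-selectable actor whose static mesh material can be swapped through options from BP_Inventory, the Game Instance.
; FindOptions borrows material UI actors by the first tag and lays them out in a row.
; ApplyOptions sets the chosen material, then parks the actors below and returns them to the inventory.
; An inventory load dispatcher replaces the base wallpaper material with the tag's stored one.
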(event `self.ReceiveBeginPlay`
  (`|ExecutionSequence`
    (:`then_0`
      ;[1 1 1] Find Inventory
      (bind _asbp_inventory (cast `/Game/Blueprints/BP_Inventory` (`GameplayStatics.GetGameInstance`)))
      (set `self.InventoryReference` _asbp_inventory))
    (:`then_1`
      (add `/Game/Blueprints/BP_Inventory.LoadInventoryDispatcher` (`self.InventoryReference`) (delegate `LoadMaterial`)))))

(event `LoadMaterial`
  (`self.LoadMaterialFromInventory`))

(event `/Game/Blueprints/BP_ObjectInterface.ApplyOptions`
  (params (CurrentUIReference :type Integer))
  ;[1 1 1] Handle Material Selection
  (if (== CurrentUIReference -1)
    (`self.ReturnUIOptions` :!label _label)
    (else
      (bind _materialinstance (`/Game/Blueprints/BP_Inventory.GetMeterialInstance` (`self.InventoryReference`) (`KismetArrayLibrary.Array_Get` (`self.UIOptions`) CurrentUIReference)))
      (if (== _materialinstance (`PrimitiveComponent.GetMaterial` (`self.StaticMesh`) 0))
        (goto _label)
        (else
          (`PrimitiveComponent.SetMaterial` (`self.StaticMesh`) 0 _materialinstance)
          (`self.ReturnUIOptions`))))))

(fn `ArrangeUIElements`
  (locals (DefaultLocaton :type "Vector Structure" :default (20.0 0.0 0.0)))
  (for (_array_element _array_index) (`self.UIOptions`)
    (`self.K2_SetActorTransform` _array_element (`KismetMathLibrary.MakeTransform` (+ (* (0.0 12.0 0.0) _array_index) (`local.DefaultLocaton`)) (`self.K2_GetActorRotation` self) (`self.GetActorScale3D` _array_element)) false false)))

(fn `FindOptions`
  (returns (Options :type "Array of /Game/Blueprints/BP_UserInterface Object Reference"))
  (bind _uireferences (`/Game/Blueprints/BP_Inventory.GetMaterialUIElements` (`self.InventoryReference`) (`KismetArrayLibrary.Array_Get` (`self.Tags`)) 0))
  (bind _output_get (set `self.UIOptions` _uireferences))
  (`self.ArrangeUIElements`)
  (return _output_get))

(fn `HasOptions`
  (returns (HasOptions :type Boolean))
  (return true))

(fn `IsSelectable`
  (returns (Selectable :type Boolean))
  (return false))

(fn `LoadMaterialFromInventory`
  (if (== (`PrimitiveComponent.GetMaterial` (`self.StaticMesh`) 0) "/Game/Materials/Floor/M_Wallpaper_Base.M_Wallpaper_Base")
    (bind _material (`/Game/Blueprints/BP_Inventory.GetMaterialReference` (`self.InventoryReference`) (`KismetArrayLibrary.Array_Get` (`self.Tags`))))
    (if (`KismetSystemLibrary.IsValid` _material)
      (`PrimitiveComponent.SetMaterial` (`self.StaticMesh`) 0 _material))))

(fn `ReturnUIOptions`
  (bind _uioptions (`self.UIOptions`))
  (for _array_element _uioptions
    (`self.K2_DetachFromActor` _array_element "KeepRelative" "KeepRelative" "KeepRelative")
    (`self.K2_SetActorLocation` _array_element (0.0 0.0 -200.0) false false))
  (`/Game/Blueprints/BP_Inventory.ReturnFurnitureUI` (`self.InventoryReference`) _uioptions))

(fn `UpdateMaterial`
  (params (TargetMaterial :type "MaterialInstanceDynamic Object Reference"))
  (for _array_element (`SceneComponent.GetChildrenComponents` (`self.DefaultSceneRoot`) false)
    (bind _asstatic_mesh_component (cast `StaticMeshComponent` _array_element))
    (`PrimitiveComponent.SetMaterial` _asstatic_mesh_component 0 (`MaterialInstance.Parent` TargetMaterial))))

(fn `UserConstructionScript`)